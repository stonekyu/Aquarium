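; BP_Target1 is a target actor that wanders in random 3D directions while its CanMove flag is set.
; A looping one-second timer started on BeginPlay picks a new random unit vector as MoveDirection.
; Tick moves the actor along that direction at MovementSpeed, scaled by delta time, using a swept SetActorLocation so blocking collision stops it.
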(event Custom|ChangeDirection
  (Variables|Default|SetMoveDirection (Math|Random|RandomUnitVector)))

(event EventBeginPlay
  (Utilities|Time|SetTimerbyEvent (delegate Custom|ChangeDirection) 1.0 true))

(event EventTick
  (params (DeltaSeconds :type Float%20%28single-precision%29))
  (if (Variables|Default|GetbCanMove)
    (Transformation|SetActorLocation (+ (Transformation|GetActorLocation) (* (Variables|Default|GetMoveDirection) (Variables|Default|GetMovementSpeed) DeltaSeconds)) true false)))

(fn ConstructionScript)