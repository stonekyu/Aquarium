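; BP_DrunkWalk is an actor that wanders in a drifting random walk, starting in a random direction.
; Each Tick rotates the direction by small, non-negative random angles on all axes, sweeps the actor along it at MovementSpeed, and faces it that way.
; The random turn is per frame, unscaled by DeltaSeconds.
; On Hit, the new direction is the impact normal reflected using the current direction as surface normal.
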(event EventBeginPlay
  (Variables|Default|SetbCanMove true)
  (Variables|Default|SetMoveDirection (Math|Random|RandomUnitVector)))

(event Collision|EventHit
  (params (MyComp :type Primitive%20Component%20Object%20Reference) (Other :type Actor%20Object%20Reference) (OtherComp :type Primitive%20Component%20Object%20Reference) (bSelfMoved :type Boolean) (HitLocation :type Vector :default "0, 0, 0") (HitNormal :type Vector :default "0, 0, 0") (NormalImpulse :type Vector :default "0, 0, 0") (Hit :type Hit%20Result%20Structure%20%28by%20ref%29))
  (Variables|Default|SetMoveDirection (Math|Vector|GetReflectionVector (.ImpactNormal (Collision|BreakHitResult Hit)) (Variables|Default|GetMoveDirection))))

(event EventTick
  (params (DeltaSeconds :type Float%20%28single-precision%29))
  (bind _returnvalue (Math|Random|RandomFloatinRange 0.0 3.0))
  (bind _returnvalue_2 (Transformation|GetActorLocation))
  (if (Variables|Default|GetbCanMove)
    (Variables|Default|SetMoveDirection (Math|Vector|RotateVector (Variables|Default|GetMoveDirection) (Math|Rotator|MakeRotator _returnvalue _returnvalue _returnvalue)))
    (Transformation|SetActorLocation (+ (Transformation|GetActorLocation) (* (Variables|Default|GetMovementSpeed) (Variables|Default|GetMoveDirection) DeltaSeconds)) true false)
    (Transformation|SetActorRotation (Math|Rotator|FindLookatRotation _returnvalue_2 (+ _returnvalue_2 (* 1e+02 (Variables|Default|GetMoveDirection)))))))

(fn ConstructionScript)