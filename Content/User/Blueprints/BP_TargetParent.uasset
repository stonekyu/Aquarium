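; BP_TargetParent is a target actor, apparently a base class, that wanders in random directions through 3D space.
; A looping timer picks a new random unit direction every second.
; While CanMove is true, Tick moves the actor along that direction at MovementSpeed with a sweep.
; On Hit, the direction becomes the impact normal reflected about the current move direction, the reverse of the usual argument order.
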(event Custom|ChangeDirection
  (Variables|Default|SetMoveDirection (Math|Random|RandomUnitVector)))

(event EventBeginPlay
  (Utilities|Time|SetTimerbyEvent (delegate Custom|ChangeDirection) 1.0 true))

(event Collision|EventHit
  (params (MyComp :type Primitive%20Component%20Object%20Reference) (Other :type Actor%20Object%20Reference) (OtherComp :type Primitive%20Component%20Object%20Reference) (bSelfMoved :type Boolean) (HitLocation :type Vector :default "0, 0, 0") (HitNormal :type Vector :default "0, 0, 0") (NormalImpulse :type Vector :default "0, 0, 0") (Hit :type Hit%20Result%20Structure%20%28by%20ref%29))
  (Variables|Default|SetMoveDirection (Math|Vector|GetReflectionVector (.ImpactNormal (Collision|BreakHitResult Hit)) (Variables|Default|GetMoveDirection))))

(event EventTick
  (params (DeltaSeconds :type Float%20%28single-precision%29))
  (if (Variables|Default|GetbCanMove)
    (Transformation|SetActorLocation (+ (Transformation|GetActorLocation) (* (Variables|Default|GetMoveDirection) (Variables|Default|GetMovementSpeed) DeltaSeconds)) true false)))

(fn ConstructionScript)