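; BP_Manta is an actor that moves a manta along a spline path.
; Each Tick advances the distance by SplineSpeed scaled by delta time, then sets the Manta component's relative transform from the spline's local-space location and rotation at that distance.
; Fixed roll and yaw offsets adjust its orientation while its scale is preserved.
; When Loop is enabled, the distance resets to zero after passing the spline's end.
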(event EventBeginPlay)

(event EventTick
  (params (DeltaSeconds :type Float%20%28single-precision%29))
  (Variables|Default|SetDistance%20Along%20Spline (+ (* DeltaSeconds (Variables|Default|GetSpline%20Speed)) (Variables|Default|GetDistance%20Along%20Spline)))
  (Transformation|SetRelativeTransform (Variables|Default|GetManta) (Math|Transform|MakeTransform (.location (Spline|GetTransformatDistanceAlongSpline (Variables|Default|GetSpline) (Variables|Default|GetDistance%20Along%20Spline) "Local" false)) (Math|Rotator|MakeRotator (+ (.roll (.rotation (Spline|GetTransformatDistanceAlongSpline (Variables|Default|GetSpline) (Variables|Default|GetDistance%20Along%20Spline) "Local" false))) 9e+01) (.pitch (.rotation (Spline|GetTransformatDistanceAlongSpline (Variables|Default|GetSpline) (Variables|Default|GetDistance%20Along%20Spline) "Local" false))) (+ (.yaw (.rotation (Spline|GetTransformatDistanceAlongSpline (Variables|Default|GetSpline) (Variables|Default|GetDistance%20Along%20Spline) "Local" false))) -9e+01)) (Variables|/Script/Engine.SceneComponent|GetRelativeScale3D (Variables|Default|GetManta))) false false)
  (if (Variables|Default|Getloop)
    (if (> (Variables|Default|GetDistance%20Along%20Spline) (Spline|GetSplineLength (Variables|Default|GetSpline)))
      (Variables|Default|SetDistance%20Along%20Spline 0.0))))

(fn ConstructionScript)